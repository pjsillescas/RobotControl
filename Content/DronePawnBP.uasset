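; Drone pawn Blueprint that drives its mesh with physics forces from four rotors.
; Each tick it takes front, back, left and right forces from GetRotorForces, which is defined outside this graph.
; A helper function applies each force to the mesh at the world location of the matching arrow component, so the arrows serve as rotor positions.
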(event `self.ReceiveTick`
  (params (DeltaSeconds :type "Float (single-precision)"))
  (bind (_frontforce _backforce _leftforce _rightforce) (`self.GetRotorForces`))
  (`self.AddForceToArrow` (`self.ArrowFront`) _frontforce)
  (`self.AddForceToArrow` (`self.ArrowBack`) _backforce)
  (`self.AddForceToArrow` (`self.ArrowLeft`) _leftforce)
  (`self.AddForceToArrow` (`self.ArrowRight`) _rightforce))

(fn `UserConstructionScript`)