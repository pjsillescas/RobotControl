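; Game state Blueprint for the robot control game that puts the main HUD on screen at start.
; On BeginPlay it looks up the first DronePawn in the level and, if one exists, creates a MainHud widget bound to that pawn and adds it to the viewport.
; Without a DronePawn in the level, no HUD is created.
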(event `self.ReceiveBeginPlay`
  (bind _robot (`self.FindRobotInLevel`))
  (`/Engine/EditorBlueprintResources/StandardMacros.IsValid` _robot
    (:`Is Valid`
      (bind _returnvalue (`|CreateWidget` "/Game/RobotControl/HUD/MainHud.MainHud_C" null _robot))
      (bind _output_get (set `self.MainHud` _returnvalue))
      (`UserWidget.AddToViewport` _output_get 0))))

(fn `FindRobotInLevel`
  (returns (Robot :type "DronePawn Object Reference"))
  (locals (LocalRobot :type "DronePawn Object Reference"))
  (bind _outactors (`GameplayStatics.GetAllActorsOfClass` "/Script/RoboticsControl.DronePawn"))
  (if (> (`KismetArrayLibrary.Array_Length` _outactors) 0)
    (set `local.LocalRobot` (`|GetArrayItem` _outactors))
    (else
      (set `local.LocalRobot` null)))
  (return (`local.LocalRobot`)))

(fn `UserConstructionScript`)